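; Chained crate actor, apparently helicopter cargo, that can break on impact or be dropped as a parachute crate.
; Non-helicopter hits pass through a DoOnce, re-armed by a half-second timer, and recompute Health from Cube speed relative to MaxHitForce, or break the crate.
; BreakCrate detaches and destroys the actor.
; DropCrate first spawns BP_ParachuteCrate at the Cube's transform with its velocity, then calls BreakCrate.
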(event `self.ReceiveBeginPlay`
  (set `self.Health` (`self.MaxHealth`)))

(event `ResetCrateCollision`
  (bind _returnvalue (`KismetMathLibrary.Lerp` (`self.MaxHealth`) 10.0 (/ (`KismetMathLibrary.VSize` (`SceneComponent.GetComponentVelocity` (`self.Cube`))) (`self.MaxHitForce`))))
  (bind _returnvalue_2 (- _returnvalue (`self.Health`)))
  (goto _label :!via `Reset`))

(event `self.Cube.OnComponentHit`
  (params (HitComponent :type "PrimitiveComponent Object Reference") (OtherActor :type "Actor Object Reference") (OtherComp :type "PrimitiveComponent Object Reference") (NormalImpulse :type "Vector Structure") (Hit :type "HitResult Structure (by ref)"))
  (bind _returnvalue (`KismetMathLibrary.Lerp` (`self.MaxHealth`) 10.0 (/ (`KismetMathLibrary.VSize` (`SceneComponent.GetComponentVelocity` (`self.Cube`))) (`self.MaxHitForce`))))
  (bind _returnvalue_2 (- _returnvalue (`self.Health`)))
  (cast `/Game/Blueprints/BP_PlayerHelicopter` OtherActor
    (:`CastFailed`
      (`/Engine/EditorBlueprintResources/StandardMacros.DoOnce` false :!label _label
        (:`Completed`
          (if (<= _returnvalue _returnvalue_2)
            (`self.BreakCrate`)
            (else
              (set `self.Health` _returnvalue_2)
              (`KismetSystemLibrary.K2_SetTimerDelegate` (delegate `ResetCrateCollision`) 0.5))))))))

(event `BreakCrate`
  (`self.K2_DetachFromActor` "KeepRelative")
  (`self.K2_DestroyActor`))

(event `DropCrate`
  (bind _cube (`self.Cube`))
  (bind _returnvalue (`|SpawnActorFromClass` "/Game/Blueprints/BP_ParachuteCrate.BP_ParachuteCrate_C" (`SceneComponent.K2_GetComponentToWorld` _cube) "Undefined" "MultiplyWithRoot" null null))
  (`PrimitiveComponent.SetPhysicsLinearVelocity` (`/Game/Blueprints/BP_ParachuteCrate.Cube` _returnvalue) (`SceneComponent.GetComponentVelocity` _cube) false "None")
  (`self.BreakCrate`))

(fn `UserConstructionScript`)