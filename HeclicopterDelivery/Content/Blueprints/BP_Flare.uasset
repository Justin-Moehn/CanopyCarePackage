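; BP_Flare is a flare actor that bobs continuously between its spawn location and a point directly above it.
; BeginPlay caches both endpoints and calls MoveFlare, where a FlipFlop alternates playing and reversing a timeline.
; The timeline's track drives a vector lerp of the actor's location without sweeping, and its Finished output calls MoveFlare again to keep the cycle going.
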(event `self.ReceiveBeginPlay`
  (bind (_returnvalue_x _returnvalue_y _returnvalue_z) (`KismetMathLibrary.BreakVector` (`self.K2_GetActorLocation`)))
  (bind (_returnvalue_x_2 _returnvalue_y_2 _returnvalue_z_2) (`KismetMathLibrary.BreakVector` (`self.K2_GetActorLocation`)))
  (set `self.DownLocation` (`KismetMathLibrary.MakeVector` _returnvalue_x_2 _returnvalue_y_2 _returnvalue_z_2))
  (set `self.UpLocation` (`KismetMathLibrary.MakeVector` _returnvalue_x _returnvalue_y (+ _returnvalue_z 500.0)))
  (`self.MoveFlare`))

(event `MoveFlare`
  (`/Engine/EditorBlueprintResources/StandardMacros.FlipFlop`
    (:`A`
      (bind (_direction _newtrack_0) (`Timeline|Timeline` :!label _label)
        (:`Update`
          (`self.K2_SetActorLocation` (`KismetMathLibrary.VLerp` (`self.DownLocation`) (`self.UpLocation`) _newtrack_0)))
        (:`Finished`
          (`self.MoveFlare`))))
    (:`B`
      (goto _label :!via `Reverse`))))

(fn `UserConstructionScript`)