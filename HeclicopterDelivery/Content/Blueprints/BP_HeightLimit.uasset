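; BP_HeightLimit is a boundary volume that pushes the player helicopter back when it strays into an out-of-bounds area.
; It caches the player helicopter on BeginPlay, and its Box overlap events set and clear an OutOfBounds flag for that helicopter class.
; While the flag is set, Tick applies a fixed world-space force to the helicopter's capsule, strongly along positive Y and slightly downward.
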(event `self.ReceiveBeginPlay`
  (bind _asbp_player_helicopter (cast `/Game/Blueprints/BP_PlayerHelicopter` (`GameplayStatics.GetPlayerCharacter` 0)))
  (set `self.As BP Player Helicopter` _asbp_player_helicopter))

(event `self.ReceiveTick`
  (params (DeltaSeconds :type "Float (single-precision)"))
  (if (`self.OutOfBounds`)
    (`PrimitiveComponent.AddForce` (`Character.CapsuleComponent` (`self.As BP Player Helicopter`)) (0.0 2100000.0 -100000.0) "None" false)))

(event `self.Box.OnComponentBeginOverlap`
  (params (OverlappedComponent :type "PrimitiveComponent Object Reference") (OtherActor :type "Actor Object Reference") (OtherComp :type "PrimitiveComponent Object Reference") (OtherBodyIndex :type Integer) (bFromSweep :type Boolean) (SweepResult :type "HitResult Structure (by ref)"))
  (cast `/Game/Blueprints/BP_PlayerHelicopter` OtherActor)
  (set `self.OutOfBounds` true))

(event `self.Box.OnComponentEndOverlap`
  (params (OverlappedComponent :type "PrimitiveComponent Object Reference") (OtherActor :type "Actor Object Reference") (OtherComp :type "PrimitiveComponent Object Reference") (OtherBodyIndex :type Integer))
  (cast `/Game/Blueprints/BP_PlayerHelicopter` OtherActor)
  (set `self.OutOfBounds` false))

(fn `UserConstructionScript`)