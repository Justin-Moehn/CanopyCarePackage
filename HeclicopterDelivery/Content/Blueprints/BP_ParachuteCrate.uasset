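; BP_ParachuteCrate is a physics crate that deploys a parachute effect while falling.
; A timer after BeginPlay plays a timeline that raises the Cube's linear and angular damping to slow it, while scaling up the Arrow component as the apparent chute.
; Any hit on the Cube reverses that timeline from its end, removing the damping and shrinking the Arrow.
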(event `self.ReceiveBeginPlay`
  (`KismetSystemLibrary.K2_SetTimerDelegate` (delegate `StartParachute`) 1.5))

(event `StartParachute`
  (bind _cube (`self.Cube`))
  (bind (_direction _newtrack_0) (`Timeline|Timeline` :!via `PlayFromStart` :!label _label)
    (:`Update`
      (`PrimitiveComponent.SetLinearDamping` _cube (`KismetMathLibrary.Lerp` 0.0 1.0 _newtrack_0))
      (`PrimitiveComponent.SetAngularDamping` _cube (`KismetMathLibrary.Lerp` 0.0 1.0 _newtrack_0))
      (bind _returnvalue (`KismetMathLibrary.Lerp` 0.01 1.0 _newtrack_0))
      (`SceneComponent.SetRelativeScale3D` (`self.Arrow`) (`KismetMathLibrary.MakeVector` _returnvalue _returnvalue _returnvalue)))))

(event `self.Cube.OnComponentHit`
  (params (HitComponent :type "PrimitiveComponent Object Reference") (OtherActor :type "Actor Object Reference") (OtherComp :type "PrimitiveComponent Object Reference") (NormalImpulse :type "Vector Structure") (Hit :type "HitResult Structure (by ref)"))
  (goto _label :!via `ReverseFromEnd`))

(fn `UserConstructionScript`)