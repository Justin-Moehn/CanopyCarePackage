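; Player helicopter that flies on physics, carries a droppable chained supply crate and takes collision damage.
; Tick ramps upward force on the capsule, traces for ground contact, and updates camera, compass and crate prompts.
; Enhanced Input drives lift, yaw look and timer-ticked pitch/roll, while timelines handle force falloff and looping blade spin.
; Debounced non-Base hits reduce health and add smoke; death spins blades down to a death screen, where resupply input reloads the level.
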(event `self.ReceiveBeginPlay`
  (bind _capsulecomponent (`self.CapsuleComponent`))
  (bind _returnvalue (`|SpawnActorFromClass` "/Game/Blueprints/BP_PlayerCamera.BP_PlayerCamera_C" (`SceneComponent.K2_GetComponentToWorld` (`self.CapsuleComponent`)) "Undefined" "MultiplyWithRoot" null self null))
  (set `self.CameraActor` _returnvalue)
  (`PrimitiveComponent.SetLinearDamping` _capsulecomponent 0.5)
  (`PrimitiveComponent.SetAngularDamping` _capsulecomponent 2.0)
  (set `self.UpForceIncreaseAMT` (/ (`self.MaxUpForce`) 20.0))
  (`self.SpinBlades` 0.0))

(event `BladeWindUp`
  (bind (_direction _newtrack_0) (`Timeline|Timeline_1` :!via `PlayFromStart` :!label _label)
    (:`Update`
      (`TimelineComponent.SetPlayRate` (`self.Timeline_0`) (`KismetMathLibrary.Lerp` 1.5 3.0 _newtrack_0)))))

(event `BladeWindDown`
  (goto _label :!via `ReverseFromEnd`))

(event `EnhancedInput|/Game/InputActions/IA_UpFlight`
  (params (ActionValue :type "Float (double-precision)") (ElapsedSeconds :type "Float (double-precision)") (TriggeredSeconds :type "Float (double-precision)") (InputAction :type "InputAction Object Reference" :default "/Game/InputActions/IA_UpFlight.IA_UpFlight"))
  (:`Triggered`
    (set `self.FlightIAValue'` ActionValue))
  (:`Started`
    (set `self.IsUpForce` true)
    (`self.BladeWindUp`))
  (:`Completed`
    (set `self.IsUpForce` false)
    (`self.BladeWindDown`)
    (bind (_direction _newtrack_0) (`Timeline|Timeline` :!via `PlayFromStart` :!label _label_2)
      (:`Update`
        (set `self.UpForce` (`KismetMathLibrary.Lerp` (`self.UpForceIncreaseAMT`) 0.0 _newtrack_0))))))

(event `CancelWindDown`
  (goto _label_2 :!via `Stop`))

(event `EnhancedInput|/Game/InputActions/IA_Rotation`
  (params (ActionValue :type "Vector2D Structure") (ElapsedSeconds :type "Float (double-precision)") (TriggeredSeconds :type "Float (double-precision)") (InputAction :type "InputAction Object Reference" :default "/Game/InputActions/IA_Rotation.IA_Rotation"))
  (bind (_x _y) (`KismetMathLibrary.BreakVector2D` ActionValue))
  (:`Triggered`
    (set `self.FlightRotationY` _y)
    (set `self.FlightRotationX` _x))
  (:`Started`
    (if (`self.IsTouchingGround`)
      _
      (elif (not (`self.IsDead`))
        (bind _returnvalue (`KismetSystemLibrary.K2_SetTimerDelegate` (delegate `RotationTick`) (`self.RotationTickTime`) true))
        (set `self.FlightRottionTimer` _returnvalue))))
  (:`Completed`
    (`KismetSystemLibrary.K2_ClearAndInvalidateTimerHandle` (`self.FlightRottionTimer`))))

(event `RotationTick`
  (bind _returnvalue (`self.FlightRotation` (`self.FlightRotationX`) (`self.FlightRotationY`)))
  (set `self.LastRotation` _returnvalue))

(event `self.ReceiveTick`
  (params (DeltaSeconds :type "Float (single-precision)"))
  (bind _maxupforce (`self.MaxUpForce`))
  (bind _capsulecomponent (`self.CapsuleComponent`))
  (bind _compass (`self.Compass`))
  (bind _capsulecomponent_2 (`self.CapsuleComponent`))
  (bind _pickupui (`self.PickUpUI`))
  (bind _dropcrateui (`self.DropCrateUI`))
  (bind _backturnpos (`self.BackTurnPos`))
  (bind (_returnvalue_roll _returnvalue_pitch _returnvalue_yaw) (`KismetMathLibrary.BreakRotator` (`SceneComponent.K2_GetComponentRotation` _capsulecomponent_2)))
  (bind _returnvalue (`SceneComponent.K2_GetComponentLocation` _backturnpos))
  (bind _defaultsceneroot (`/Game/Blueprints/BP_PlayerCamera.DefaultSceneRoot` (`self.CameraActor`)))
  (bind (_returnvalue_roll_2 _returnvalue_pitch_2 _returnvalue_yaw_2) (`KismetMathLibrary.BreakRotator` (`KismetMathLibrary.FindLookAtRotation` (`SceneComponent.K2_GetComponentLocation` _defaultsceneroot) (`SceneComponent.K2_GetComponentLocation` (`self.LeftTurnPos`)))))
  (`/Engine/EditorBlueprintResources/StandardMacros.IsValid` (`self.CrateActor`)
    (:`Is Valid`
      _)
    (:`Is Not Valid`
      (`/Engine/EditorBlueprintResources/StandardMacros.IsValid` _dropcrateui
        (:`Is Valid`
          (`Widget.RemoveFromParent` _dropcrateui))
        (:`Is Not Valid`
          _))))
  (if (and (`self.PositionToResupply`) (not (`KismetSystemLibrary.IsValid` (`self.CrateActor`))))
    (`/Engine/EditorBlueprintResources/StandardMacros.IsValid` (`self.PickUpUI`)
      (:`Is Valid`
        _)
      (:`Is Not Valid`
        (bind _returnvalue_2 (`|CreateWidget` "/Game/UI/WB_PickUpButtom.WB_PickUpButtom_C"))
        (set `self.PickUpUI` _returnvalue_2)
        (`UserWidget.AddToViewport` _returnvalue_2 0)))
    (else
      (`/Engine/EditorBlueprintResources/StandardMacros.IsValid` _pickupui
        (:`Is Valid`
          (`Widget.RemoveFromParent` _pickupui)
          (set `self.PickUpUI` null))
        (:`Is Not Valid`
          _))))
  (if (not (`self.IsDead`))
    (`SceneComponent.K2_SetWorldRotation` _compass (`KismetMathLibrary.MakeRotator` 0.0 90.0 _returnvalue_yaw) false false)
    (`SceneComponent.K2_SetWorldLocation` _compass (`SceneComponent.K2_GetComponentLocation` _capsulecomponent_2) false true)
    (if (not (`self.IsLooking`))
      (`SceneComponent.K2_SetWorldRotation` _defaultsceneroot (`KismetMathLibrary.MakeRotator` 0.0 0.0 (+ _returnvalue_yaw_2 -90.0)) false false))
    (bind (_outhit _returnvalue_3) (`KismetSystemLibrary.LineTraceSingle` _returnvalue (+ _returnvalue (* (* (`SceneComponent.GetForwardVector` _backturnpos) -1.0) 250.0)) "TraceTypeQuery1" false (`self.Actors to Ignore`)))
    (if (and _returnvalue_3 (not (`self.IsUpForce`)))
      (set `self.IsTouchingGround` true)
      (else
        (set `self.IsTouchingGround` false)))
    (if (`self.IsUpForce`)
      (`self.CancelWindDown`)
      (if (>= (`self.UpForce`) _maxupforce)
        (set `self.UpForce` _maxupforce)
        (else
          (set `self.UpForce` (+ (`self.UpForce`) (`self.UpForceIncreaseAMT`)))))
      (`PrimitiveComponent.AddForce` _capsulecomponent (* (`SceneComponent.GetUpVector` _capsulecomponent) (* (`self.UpForce`) (`self.FlightIAValue'`))) "None" false))))

(event `EnhancedInput|/Game/InputActions/IA_Look`
  (params (ActionValue :type "Vector2D Structure") (ElapsedSeconds :type "Float (double-precision)") (TriggeredSeconds :type "Float (double-precision)") (InputAction :type "InputAction Object Reference" :default "/Game/InputActions/IA_Look.IA_Look"))
  (bind (_x _y) (`KismetMathLibrary.BreakVector2D` ActionValue))
  (:`Triggered`
    (if (not (and (not (`self.IsDead`)) (`self.IsTouchingGround`)))
      (`self.Look` _x _y)))
  (:`Started`
    (set `self.IsLooking` true))
  (:`Completed`
    (set `self.IsLooking` false)))

(event `Update UI - Crate`
  (params (CrateState :type Integer))
  (`/Game/Blueprints/UI_cratestate.update UI` (`self.UI`) CrateState))

(event `Resupply`
  (`/Engine/EditorBlueprintResources/StandardMacros.IsValid` (`self.CrateActor`)
    (:`Is Not Valid`
      (bind _returnvalue (`|SpawnActorFromClass` "/Game/Blueprints/BP_Chain1.BP_Chain1_C" (`KismetMathLibrary.MakeTransform` (`SceneComponent.RelativeLocation` (`self.CrateAttachPoint`)) (struct :`Yaw` 90.0 :`Roll` 90.0)) "Undefined" "MultiplyWithRoot" null null))
      (bind _output_get (set `self.CrateActor` _returnvalue))
      (`self.K2_AttachToActor` _output_get self "None" "SnapToTarget" "SnapToTarget" "SnapToTarget" true)
      (`KismetArrayLibrary.Array_Add` (`self.Actors to Ignore`) _output_get)
      (`PrimitiveComponent.SetSimulatePhysics` (`/Game/Blueprints/BP_Chain1.Cube` _output_get) true)
      (bind _returnvalue_2 (`|CreateWidget` "/Game/Blueprints/UI_cratestate.UI_cratestate_C"))
      (`UserWidget.AddToViewport` _returnvalue_2 0)
      (set `self.UI` _returnvalue_2)
      (bind _returnvalue_3 (`|CreateWidget` "/Game/UI/WB_DropCrateButtom.WB_DropCrateButtom_C"))
      (set `self.DropCrateUI` _returnvalue_3)
      (`UserWidget.AddToViewport` _returnvalue_3 0))))

(event `EnhancedInput|/Game/InputActions/IA_DropCrate`
  (params (ActionValue :type Boolean) (ElapsedSeconds :type "Float (double-precision)") (TriggeredSeconds :type "Float (double-precision)") (InputAction :type "InputAction Object Reference" :default "/Game/InputActions/IA_DropCrate.IA_DropCrate"))
  (:`Started`
    (`/Engine/EditorBlueprintResources/StandardMacros.IsValid` (`self.CrateActor`)
      (:`Is Valid`
        (`/Game/Blueprints/BP_Chain1.DropCrate` (`self.CrateActor`))
        (`/Game/Blueprints/UI_cratestate.update UI` (`self.UI`) 0)))))

(event `ResetDAMAGE`
  (bind _returnvalue (- (`self.Health`) 1))
  (goto _label_3 :!via `Reset`))

(event `self.we1.OnComponentHit`
  (params (HitComponent :type "PrimitiveComponent Object Reference") (OtherActor :type "Actor Object Reference") (OtherComp :type "PrimitiveComponent Object Reference") (NormalImpulse :type "Vector Structure") (Hit :type "HitResult Structure (by ref)"))
  (bind _returnvalue (- (`self.Health`) 1))
  (if (not (`self.ActorHasTag` OtherActor "Base"))
    (`/Engine/EditorBlueprintResources/StandardMacros.DoOnce` false :!label _label_3
      (:`Completed`
        (if (> _returnvalue 0)
          (bind _output_get (set `self.Health` _returnvalue))
          (switch `int` _output_get
            (:`1`
              (`NiagaraFunctionLibrary.SpawnSystemAttached` "/Game/Niagara/NS_Smoke.NS_Smoke" (`self.CapsuleComponent`) "None" (`SceneComponent.RelativeLocation` (`self.SmokeLocation`)) (struct) "KeepRelativeOffset" :!label _label_4))
            (:`2`
              (goto _label_4))
            (:`3`
              (goto _label_4))
            (:`4`
              _))
          (`KismetSystemLibrary.K2_SetTimerDelegate` (delegate `ResetDAMAGE`) 1.0)
          (else
            (set `self.IsDead` true)
            (set `self.Health` 0)))))))

(event `EnhancedInput|/Game/InputActions/IA_Resupply`
  (params (ActionValue :type Boolean) (ElapsedSeconds :type "Float (double-precision)") (TriggeredSeconds :type "Float (double-precision)") (InputAction :type "InputAction Object Reference" :default "/Game/InputActions/IA_Resupply.IA_Resupply"))
  (:`Started`
    (if (`self.IsDead`)
      (`GameplayStatics.OpenLevelBySoftObjectPtr` "/Game/migration/level_blueprint.level_blueprint")
      (elif (`self.PositionToResupply`)
        (`self.Resupply`)))))

(event `self.we.OnComponentHit`
  (params (HitComponent :type "PrimitiveComponent Object Reference") (OtherActor :type "Actor Object Reference") (OtherComp :type "PrimitiveComponent Object Reference") (NormalImpulse :type "Vector Structure") (Hit :type "HitResult Structure (by ref)"))
  (if (not (`self.ActorHasTag` OtherActor "Base"))
    (goto _label_3)))

(event `SpinBlades`
  (params (Speed :type "Float (double-precision)"))
  (bind (_relativerotation_roll _relativerotation_pitch _relativerotation_yaw) (`KismetMathLibrary.BreakRotator` (`SceneComponent.RelativeRotation` (`self.Blades`))))
  (if (`self.IsDead`)
    (`/Engine/EditorBlueprintResources/StandardMacros.DoOnce` false
      (:`Completed`
        (bind _output_get (set `self.StartSpinDown` _relativerotation_yaw))
        (set `self.EndSpinDown` (+ _output_get 360.0))
        (bind (_direction _newtrack_0) (`Timeline|Timeline_2` :!via `PlayFromStart`)
          (:`Update`
            (`SceneComponent.K2_SetRelativeRotation` (`self.Blades`) (`KismetMathLibrary.MakeRotator` 0.0 0.0 (`KismetMathLibrary.Lerp` (`self.StartSpinDown`) (`self.EndSpinDown`) _newtrack_0)) false false))
          (:`Finished`
            (bind _returnvalue (`|CreateWidget` "/Game/UI/WB_DeathScreen.WB_DeathScreen_C"))
            (`UserWidget.AddToViewport` _returnvalue 0)))))
    (else
      (bind (_direction_2 _newtrack_0_2) (`Timeline|Timeline_0` :!via `PlayFromStart`)
        (:`Update`
          (`SceneComponent.K2_SetRelativeRotation` (`self.Blades`) (`KismetMathLibrary.MakeRotator` 0.0 0.0 (`KismetMathLibrary.Lerp` 0.0 360.0 _newtrack_0_2)) false false))
        (:`Finished`
          (`self.SpinBlades` 0.0))))))

(fn `FlightRotation`
  (params (X :type "Float (double-precision)") (Y :type "Float (double-precision)"))
  (returns (ReturnValue :type "Rotator Structure"))
  (bind _capsulecomponent (`self.CapsuleComponent`))
  (bind _rotationspeed (`self.RotationSpeed`))
  (`SceneComponent.K2_SetRelativeRotation` _capsulecomponent (`KismetMathLibrary.TransformRotation` (`SceneComponent.GetRelativeTransform` _capsulecomponent) (`KismetMathLibrary.MakeRotator` (* Y _rotationspeed) (* X _rotationspeed))) false false))

(fn `Look`
  (params (X :type "Float (double-precision)") (Y :type "Float (double-precision)"))
  (bind _capsulecomponent (`self.CapsuleComponent`))
  (bind _cameraactor (`self.CameraActor`))
  (bind (_returnvalue_roll _returnvalue_pitch _returnvalue_yaw) (`KismetMathLibrary.BreakRotator` (`SceneComponent.K2_GetComponentRotation` _capsulecomponent)))
  (bind (_returnvalue_roll_2 _returnvalue_pitch_2) (`KismetMathLibrary.BreakRotator` (`self.K2_GetActorRotation` _cameraactor)))
  (bind (_relativerotation_roll _relativerotation_pitch _relativerotation_yaw) (`KismetMathLibrary.BreakRotator` (`SceneComponent.RelativeRotation` _capsulecomponent)))
  (`SceneComponent.K2_SetRelativeRotation` _capsulecomponent (`KismetMathLibrary.MakeRotator` _relativerotation_roll _relativerotation_pitch (+ _relativerotation_yaw (* (`self.LookSensitivity`) X))) false false)
  (`SceneComponent.K2_SetWorldRotation` (`/Game/Blueprints/BP_PlayerCamera.DefaultSceneRoot` _cameraactor) (`KismetMathLibrary.MakeRotator` _returnvalue_roll_2 _returnvalue_pitch_2 _returnvalue_yaw) false false))

(fn `UserConstructionScript`)