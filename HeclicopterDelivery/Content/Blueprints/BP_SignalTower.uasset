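; BP_SignalTower is a signal tower actor with a light that blinks on and off.
; A looping timer started at BeginPlay fires every two seconds into a FlipFlop.
; Each toggle swaps visibility between the Off component and the lit set of On component, point light and local fog volume.
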(event `self.ReceiveBeginPlay`
  (`KismetSystemLibrary.K2_SetTimerDelegate` (delegate `OnOffLight`) 2.0 true))

(event `OnOffLight`
  (bind _on (`self.on`))
  (bind _off (`self.off`))
  (`/Engine/EditorBlueprintResources/StandardMacros.FlipFlop`
    (:`A`
      (`SceneComponent.SetVisibility` _on false false)
      (`SceneComponent.SetVisibility` (`self.PointLight1`) false false)
      (`SceneComponent.SetVisibility` (`self.LocalFogVolume1`) false false)
      (`SceneComponent.SetVisibility` _off true false))
    (:`B`
      (`SceneComponent.SetVisibility` _on true false)
      (`SceneComponent.SetVisibility` (`self.PointLight1`) true false)
      (`SceneComponent.SetVisibility` (`self.LocalFogVolume1`) true false)
      (`SceneComponent.SetVisibility` _off false false))))

(fn `UserConstructionScript`)